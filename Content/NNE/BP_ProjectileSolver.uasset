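; BP_ProjectileSolver is an NNE test launcher that fires projectiles at a Target actor using an AI-computed launch angle.
; A looping one-second timer passes the target's location to FireProjectileWithAI while the target is valid.
; The returned angle and target go into a spawned BP_CollectorBall with data collection turned off.
; An unconnected variant derives a launch direction from GetAILaunchParameters and rotates an arrow to match.
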(event Custom|ShootProjectile
  (bind _target (Variables|Default|GetTarget)
    (:then
      (bind _returnvalue (Class|NNEProjectileSolver|FireProjectilewithAI (Transformation|GetActorLocation _target)))
      (Game|SpawnActorfromClass "/Game/NNE/BP_CollectorBall.BP_CollectorBall_C" (Transformation|GetActorTransform) "Undefined" "MultiplyWithRoot" 0 0 _returnvalue (Variables|Default|GetTarget) false 0))
    (:else)))

(event EventBeginPlay
  (Utilities|Time|SetTimerbyEvent (delegate Custom|ShootProjectile) 1.0 true))

(fn ConstructionScript)