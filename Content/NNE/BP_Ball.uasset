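; BP_Ball is a projectile that launches toward a target location and records the launch parameters of shots that hit.
; On BeginPlay it stores its start location and applies a fixed-strength impulse along the horizontal direction to the target, pitched by Angle.
; When its collision overlaps a BP_Target, it passes horizontal distance, height difference and Angle to DataCollect as a data sample.
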(event OnComponentBeginOverlap(Collision)
  (params (OverlappedComponent :type Primitive%20Component%20Object%20Reference) (OtherActor :type Actor%20Object%20Reference) (OtherComp :type Primitive%20Component%20Object%20Reference) (OtherBodyIndex :type Integer) (bFromSweep :type Boolean) (SweepResult :type Hit%20Result%20Structure%20%28by%20ref%29))
  (Utilities|Casting|CastToBP_Target OtherActor)
  (CallFunction|SaveData))

(event EventBeginPlay
  (Variables|Default|SetStartLoc (Transformation|GetActorLocation))
  (Physics|AddImpulse (Variables|Default|GetCollision) (* (CallFunction|GetDirectionbyAngle) 5e+04) "None" false))

(fn ConstructionScript)

(fn GetDirectionbyAngle
  (bind _targetloc (Variables|Default|GetTargetLoc))
  (bind _startloc (Variables|Default|GetStartLoc))
  (bind _returnvalue (- (Math|Vector|MakeVector (.x _targetloc) (.y _targetloc) 0.0) (Math|Vector|MakeVector (.x _startloc) (.y _startloc) 0.0)))
  (bind _returnvalue_2 (Math|Vector|Normalize _returnvalue))
  (return (Math|Vector|RotateVectorAroundAxis _returnvalue_2 (Variables|Default|GetAngle) (Math|Vector|CrossProduct _returnvalue_2 "0.000000,0.000000,1.000000"))))

(fn SaveData
  (Class|DataCollectComponent|SaveProjectileData (Variables|Default|GetDataCollect) (Math|Vector|Distance2D(Vector) (Variables|Default|GetTargetLoc) (Variables|Default|GetStartLoc)) (- (.z (Variables|Default|GetTargetLoc)) (.z (Variables|Default|GetStartLoc))) (Variables|Default|GetAngle)))