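; BP_CollectorBall is a projectile that gathers launch data, apparently for neural network (NNE) aiming.
; On BeginPlay it impulses its Sphere toward Target, pitched by Angle around the horizontal perpendicular axis.
; Overlapping a BP_Target logs start location, target location and angle to DataCollector, gated by an IsCollectData validity check.
; Blocking hits or a ten-second timeout destroy it without logging, so only successful shots are recorded.
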(event OnComponentBeginOverlap(Sphere)
  (params (OverlappedComponent :type Primitive%20Component%20Object%20Reference) (OtherActor :type Actor%20Object%20Reference) (OtherComp :type Primitive%20Component%20Object%20Reference) (OtherBodyIndex :type Integer) (bFromSweep :type Boolean) (SweepResult :type Hit%20Result%20Structure%20%28by%20ref%29))
  (Utilities|Casting|CastToBP_Target OtherActor)
  (CallFunction|MakeData true)
  (Actor|DestroyActor))

(event OnComponentHit(Sphere)
  (params (HitComponent :type Primitive%20Component%20Object%20Reference) (OtherActor :type Actor%20Object%20Reference) (OtherComp :type Primitive%20Component%20Object%20Reference) (NormalImpulse :type Vector :default "0, 0, 0") (Hit :type Hit%20Result%20Structure%20%28by%20ref%29))
  (CallFunction|MakeData false)
  (Actor|DestroyActor))

(event EventBeginPlay
  (bind _returnvalue (Transformation|GetActorLocation))
  (bind _target (Variables|Default|GetTarget))
  (bind _returnvalue_2 (Transformation|GetActorLocation _target))
  (bind _returnvalue_3 (- _returnvalue_2 _returnvalue))
  (bind _returnvalue_4 (Math|Vector|Normalize _returnvalue_3))
  (Variables|Default|SetStartTransform (Transformation|GetActorTransform))
  (Physics|AddImpulse (Variables|Default|GetSphere) (* (Math|Vector|RotateVectorAroundAxis _returnvalue_4 (Variables|Default|GetAngle) (Math|Vector|CrossProduct _returnvalue_4 "0.000000,0.000000,1.000000")) 1e+05) "None" false)
  (Utilities|FlowControl|Delay 1e+01)
  (Actor|DestroyActor))

(fn ConstructionScript)

(fn MakeData
  (params (bIsHit :type Boolean))
  (if bIsHit
    (Variables|Default|GetIsCollectData
      (:then
        (Class|NNEDataCollector|LogProjectileData (Variables|Default|GetDataCollector) (.location (Variables|Default|GetStartTransform)) (Transformation|GetActorLocation (Variables|Default|GetTarget)) (Variables|Default|GetAngle) bIsHit)
        (Development|PrintString "Collect Data"))
      (:else))))