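; BP_NNEDataCollector is a spawner actor that repeatedly launches BP_CollectorBall actors for a Target, apparently to gather data for NNE.
; While the Target is valid, a fast looping timer moves the collector to a random X and Z position before each spawn.
; Each ball receives the collector, the Target and a random angle.
; A helper computes a direction facing the Target with randomized pitch.
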(event Custom|SpawnBall
  (CallFunction|RandomNewLocaiton)
  (Game|SpawnActorfromClass "/Game/NNE/BP_CollectorBall.BP_CollectorBall_C" (Transformation|GetActorTransform) "Undefined" "MultiplyWithRoot" 0 self (Math|Random|RandomFloatinRange -1e+01 6e+01) (Variables|Default|GetTarget) true 0))

(event EventBeginPlay
  (Variables|Default|GetTarget
    (:then
      (Utilities|Time|SetTimerbyEvent (delegate Custom|SpawnBall) 0.05 true))
    (:else)))

(fn ConstructionScript)

(fn RandomNewLocaiton
  (Transformation|SetActorLocation (Math|Vector|MakeVector (Math|Random|RandomFloatinRange -3e+03 5e+02) 0.0 (Math|Random|RandomFloatinRange 5e+01 1e+03)) false false))

(fn GetRandomDirection
  (params (Min :type Float%20%28double-precision%29) (Max :type Float%20%28double-precision%29))
  (bind _returnvalue (Transformation|GetActorLocation))
  (bind _target (Variables|Default|GetTarget))
  (bind _returnvalue_2 (Transformation|GetActorLocation _target))
  (bind _returnvalue_3 (Math|Rotator|FindLookatRotation _returnvalue _returnvalue_2))
  (return (Math|Vector|GetForwardVector (Math|Rotator|MakeRotator (.roll _returnvalue_3) (Math|Random|RandomFloatinRange Min Max) (.yaw _returnvalue_3)))))