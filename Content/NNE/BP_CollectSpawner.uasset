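; BP_CollectSpawner is a spawner actor that rapidly fires off BP_Ball actors around a Target on a fast looping timer started at BeginPlay.
; Before each spawn, RandomLocation moves the spawner along its horizontal bearing from the Target to a random distance, with a random height offset.
; Each ball spawns at the spawner's transform and receives the Target's location and a random angle.
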(event Custom|SpawnBall
  (CallFunction|RandomLocation)
  (Game|SpawnActorfromClass "/Game/NNE/BP_Ball.BP_Ball_C" (Transformation|GetActorTransform) "Undefined" "MultiplyWithRoot" 0 (Transformation|GetActorLocation (Variables|Default|GetTarget)) (Math|Random|RandomFloatinRange -1e+01 6e+01) 0))

(event EventBeginPlay
  (Utilities|Time|SetTimerbyEvent (delegate Custom|SpawnBall) 0.02 true))

(fn ConstructionScript)

(fn RandomLocation
  (bind _returnvalue (Transformation|GetActorLocation))
  (bind _target (Variables|Default|GetTarget))
  (bind _returnvalue_2 (Transformation|GetActorLocation _target))
  (LocalVariables|SetRandDist (Math|Random|RandomFloatinRange 1e+02 3e+03))
  (LocalVariables|SetRandZ (Math|Random|RandomFloatinRange -1e+02 5e+02))
  (Transformation|SetActorLocation (Math|Vector|MakeVector (.x (+ (Transformation|GetActorLocation (Variables|Default|GetTarget)) (* (Math|Vector|GetForwardVector (Math|Rotator|FindLookatRotation (Math|Vector|MakeVector (.x _returnvalue_2) (.y _returnvalue_2) 0.0) (Math|Vector|MakeVector (.x _returnvalue) (.y _returnvalue) 0.0))) (LocalVariables|GetRandDist)))) (.y (+ (Transformation|GetActorLocation (Variables|Default|GetTarget)) (* (Math|Vector|GetForwardVector (Math|Rotator|FindLookatRotation (Math|Vector|MakeVector (.x _returnvalue_2) (.y _returnvalue_2) 0.0) (Math|Vector|MakeVector (.x _returnvalue) (.y _returnvalue) 0.0))) (LocalVariables|GetRandDist)))) (- (.z (+ (Transformation|GetActorLocation (Variables|Default|GetTarget)) (* (Math|Vector|GetForwardVector (Math|Rotator|FindLookatRotation (Math|Vector|MakeVector (.x _returnvalue_2) (.y _returnvalue_2) 0.0) (Math|Vector|MakeVector (.x _returnvalue) (.y _returnvalue) 0.0))) (LocalVariables|GetRandDist)))) (LocalVariables|GetRandZ))) false false))