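; Spawner actor that launches a BP_Ball toward a Target on a looping one-second timer.
; Each spawn uses the spawner's transform and passes the target's location and a launch angle to the ball.
; GetAIAngle obtains that angle from SmartAngle, feeding it the horizontal distance and height difference between spawner and target.
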(event Custom|SpawnBall
  (Game|SpawnActorfromClass "/Game/NNE/BP_Ball.BP_Ball_C" (Transformation|GetActorTransform) "Undefined" "MultiplyWithRoot" 0 (Transformation|GetActorLocation (Variables|Default|GetTarget)) (CallFunction|GetAIAngle) 0))

(event EventBeginPlay
  (Utilities|Time|SetTimerbyEvent (delegate Custom|SpawnBall) 1.0 true))

(fn ConstructionScript)

(fn GetAIAngle
  (bind _returnvalue (Class|SmartAngleComponent|GetSmartAngle (Variables|Default|GetSmartAngle) (Math|Vector|Distance2D(Vector) (Transformation|GetActorLocation (Variables|Default|GetTarget)) (Transformation|GetActorLocation)) (- (.z (Transformation|GetActorLocation (Variables|Default|GetTarget))) (.z (Transformation|GetActorLocation)))))
  (return _returnvalue))